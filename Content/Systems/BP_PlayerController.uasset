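; Player controller that adds the crosshair HUD on BeginPlay and handles the mouse cursor and inventory toggles.
; IA_Inventory creates and shows WBP_Inventory, or removes it if the stored reference is valid, calling ShowCursor either way.
; ShowCursor is a FlipFlop between Game and UI input with cursor and Game Only without it.
; IA_ShowMouse shares that FlipFlop, so cursor state can fall out of step with inventory visibility.
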(event `self.ReceiveBeginPlay`
  (bind _returnvalue (`|CreateWidget` "/Game/UI/WBP_Crosshair.WBP_Crosshair_C"))
  (`UserWidget.AddToViewport` _returnvalue 0))

(event `EnhancedInput|/Game/Systems/Input/Actions/IA_ShowMouse`
  (params (ActionValue :type Boolean) (ElapsedSeconds :type "Float (double-precision)") (TriggeredSeconds :type "Float (double-precision)") (InputAction :type "InputAction Object Reference" :default "/Game/Systems/Input/Actions/IA_ShowMouse.IA_ShowMouse"))
  (:`Started`
    (`self.ShowCursor`)))

(event `ShowCursor`
  (`/Engine/EditorBlueprintResources/StandardMacros.FlipFlop`
    (:`A`
      (`WidgetBlueprintLibrary.SetInputMode_GameAndUIEx` self null "DoNotLock" false true)
      (set `self.bShowMouseCursor` true))
    (:`B`
      (`WidgetBlueprintLibrary.SetInputMode_GameOnly` self true)
      (set `self.bShowMouseCursor` false))))

(event `EnhancedInput|/Game/Systems/Input/Actions/IA_Inventory`
  (params (ActionValue :type Boolean) (ElapsedSeconds :type "Float (double-precision)") (TriggeredSeconds :type "Float (double-precision)") (InputAction :type "InputAction Object Reference" :default "/Game/Systems/Input/Actions/IA_Inventory.IA_Inventory"))
  (:`Started`
    (`self.Ref Inventory`
      (:`then`
        (`Widget.RemoveFromParent` (`self.Ref Inventory`))
        (set `self.Ref Inventory` null)
        (`self.ShowCursor`))
      (:`else`
        (bind _returnvalue (`|CreateWidget` "/Game/UI/WBP_Inventory.WBP_Inventory_C"))
        (bind _output_get (set `self.Ref Inventory` _returnvalue))
        (`UserWidget.AddToViewport` _output_get 0)
        (`self.ShowCursor`)))))

(fn `UserConstructionScript`)